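; Game mode for a timed checkpoint race, where crossing the finish line wins and running out of time loses.
; On BeginPlay it binds events on every BP_Checkpoint, split by finish line or not, then runs a countdown before starting the time-limit timer.
; Checkpoint crossings set the timer to the starting duration plus the bonus, ignoring time remaining.
; Win and loss are only printed to screen.
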(event Custom|Game%20Finish
  (params (Win :type Boolean))
  (Development|PrintString (Utilities|String|SelectString "You Win" "You Lose" Win)))

(event Custom|Start%20Countdown
  (Development|PrintString "Start Countdown")
  (Utilities|FlowControl|Delay (Variables|Default|GetStartCountdownDuration))
  (CallFunction|GameStart))

(event Custom|CrossedACheckpoint
  (params (TimeToAdd :type Integer))
  (CallFunction|AddTimetoTimer TimeToAdd))

(event Custom|Game%20Start
  (Development|PrintString "Game has Started")
  (bind _returnvalue (Utilities|Time|SetTimerbyEvent (delegate Custom|Lose_OutOfTime) (Variables|Default|GetStartTimerDuration)))
  (Variables|Default|SetTimeRemainingTimer _returnvalue))

(event Custom|Lose_OutOfTime
  (CallFunction|GameFinish false))

(event Custom|Win_CrossTheFinishLine
  (Utilities|Time|ClearandInvalidateTimerbyHandle (Variables|Default|GetTimeRemainingTimer))
  (CallFunction|GameFinish true))

(event EventBeginPlay
  (Utilities|FlowControl|Sequence
    (:then_0
      (bind _outactors (Actor|GetAllActorsOfClass "/Game/RacingGame/Checkpoints/BP_Checkpoint.BP_Checkpoint_C"))
      (for _array_element _outactors
        (if (Variables|/Game/RacingGame/Checkpoints/BP_Checkpoint.BP_Checkpoint_C|GetIsFinishLine _array_element)
          (EventDispatchers|BindEventtoOnCheckpointCrossed _array_element (EventDispatchers|CreateEvent :!event Custom|Win_CrossTheFinishLine))
          (else
            (EventDispatchers|BindEventtoOnCheckpointCrossedwithTime _array_element (EventDispatchers|CreateEvent :!event Custom|CrossedACheckpoint))))))
    (:then_1
      (CallFunction|StartCountdown))))

(event EventTick
  (params (DeltaSeconds :type Float%20%28single-precision%29)))

(fn ConstructionScript)

(fn AddTimetoTimer
  (params (TimeToAdd :type Integer))
  (bind _returnvalue (Utilities|Time|SetTimerbyEvent (EventDispatchers|CreateEvent :!event Custom|Lose_OutOfTime) (+ (Variables|Default|GetStartTimerDuration) TimeToAdd)))
  (Variables|Default|SetTimeRemainingTimer _returnvalue))